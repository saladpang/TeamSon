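; Sword hidden-object actor for the SPROUTS set, with a Rocks component that serves as its highlightable, hideable visual.
; Clicking hides Rocks, plays a click sound and spawns the sword label actor at its location; a cursor-over event also hides Rocks.
; Tick uses screen projection success as a visibility test, applying a highlight material once after a delay, then restoring the basic material and re-arming when projection fails.
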(event Custom|OnBeginCursorOver_Event_0
  (params (TouchedActor :type Actor%20Object%20Reference))
  (Development|SetHiddeninGame (Variables|Default|GetRocks) true false))

(event MouseInput|EventActorOnClicked
  (params (ButtonPressed :type Key%20Structure :default "None"))
  (bind _returnvalue (Transformation|GetActorLocation))
  (Development|SetHiddeninGame (Variables|Default|GetRocks) true false)
  (Audio|PlaySoundatLocation "/Game/HiddenObjects_TS/SPROUTS/click.click" _returnvalue "0, 0, 0" 1.0 1.0 0.0 0 0 0)
  (Game|SpawnActorfromClass "/Game/HiddenObjects_TS/SPROUTS/BP_Label_Sword_SPROUTS.BP_Label_Sword_SPROUTS_C" (Math|Conversions|ToTransform(Vector) _returnvalue) "Undefined" 0 0))

(event EventTick
  (params (DeltaSeconds :type Float%20%28single-precision%29))
  (bind _rocks (Variables|Default|GetRocks))
  (if (.ReturnValue (Class|GameplayStatics|ProjectWorldtoScreen (Game|GetPlayerController 0) (Transformation|GetActorLocation) false))
    (Utilities|FlowControl|DoOnce false :!label _label
      (:Completed
        (Utilities|FlowControl|Delay 2.0)
        (Rendering|Material|SetMaterial _rocks 0 "/Game/ExampleContent/Blueprint_Communication/Materials/M_Orange_Shiny_Highlighted.M_Orange_Shiny_Highlighted")))
    (else
      (Rendering|Material|SetMaterial _rocks 0 "/Engine/BasicShapes/BasicShapeMaterial.BasicShapeMaterial")
      (goto _label Reset))))

(fn ConstructionScript)